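; Player character for a cursor-aimed shooter with three weapon slots, magic attacks and a limited-charge dash.
; Tick traces under the mouse to turn the character toward the cursor.
; Fire and Magic spawn slot-specific projectiles through ShootProjectile, sharing ammo with automatic reload, except slot three's magic, which latches on a flamethrower.
; Acid debuff re-triggers itself to slow and replay effects, while damage intake and other received debuffs are unfinished.
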(event `RadiationDebuff_1_1`
  (params (Entered :type Boolean)))

(event `Key|R`
  (params (Key :type "Key Structure"))
  ;[1 1 1] Weapon Swap
  (:`Pressed`
    (`self.Reloading`)))

(event `self.ReceiveTick`
  (params (DeltaSeconds :type "Float (single-precision)"))
  ;[1 0 0.178] Event Tick
  (`self.RotateFunc`)
  (if (`self.FlameThrowerActivate`)
    (`self.Flame Thrower Emitter`)))

(event `Key|One`
  (params (Key :type "Key Structure"))
  ;[1 1 1] Weapon Swap
  (:`Pressed`
    (set `self.Weapon_Number` 1)))

(event `/Game/BP/Blueprints/Combat/BP_Debuff_Interfacer.AcidDebuff`
  (params (CountAnim :type Integer) (AnimTime :type "Float (single-precision)"))
  (`self.CustomEvent_0` 5))

(event `Key|Two`
  (params (Key :type "Key Structure"))
  ;[1 1 1] Weapon Swap
  (:`Pressed`
    (set `self.Weapon_Number` 2)))

(event `Key|Three`
  (params (Key :type "Key Structure"))
  ;[1 1 1] Weapon Swap
  (:`Pressed`
    (set `self.Weapon_Number` 3)))

(event `ShootState`
  ;[1 1 1] ShootState
  (set `self.bIsShooting` true)
  (`KismetSystemLibrary.RetriggerableDelay` 0.2)
  (set `self.bIsShooting` false))

(event `CustomEvent_0`
  (params (CountAnim :type Integer) (AnimTime :type "Float (double-precision)"))
  (`self.Debuf` 300.0 0.0)
  (`self.PlayEffect` null "/Game/BP/Blueprints/Combat/AcidNiagara.AcidNiagara")
  (bind _output_get (set `self.Count Anim` (- CountAnim 1)))
  (if (>= _output_get 0)
    (`KismetSystemLibrary.Delay` 2.0)
    (`self.CustomEvent_0` _output_get)))

(event `self.ReceiveAnyDamage`
  (params (Damage :type "Float (single-precision)") (DamageType :type "DamageType Object Reference") (InstigatedBy :type "Controller Object Reference") (DamageCauser :type "Actor Object Reference"))
  ;[1 1 1] Recive damage
)

(event `/Game/BP/Blueprints/Combat/BP_Debuff_Interfacer.ElectroDebuff`)

(event `InputAction|Fire`
  (params (Key :type "Key Structure"))
  (bind _returnvalue (`SceneComponent.K2_GetComponentRotation` (`self.Arrow1`)))
  ;[1 1 1] Shooting
  (:`Pressed`
    (switch `int` (`self.Weapon_Number`)
      (:`Default`
        (`self.Shoot Projectile` 5.0 "/Game/BP/Blueprints/Combat/BP_Basic_Bullet.BP_Basic_Bullet_C" (0.2 0.2 0.2) _returnvalue :!label _label))
      (:`1`
        (goto _label))
      (:`2`
        (`self.Shoot Projectile` 15.0 "/Game/BP/Blueprints/Combat/BP_Basic_Bullet_2.BP_Basic_Bullet_2_C" (0.25 0.25 0.25) _returnvalue))
      (:`3`
        (`self.Shoot Projectile` 25.0 "/Game/BP/Blueprints/Combat/BP_Basic_Bullet_3.BP_Basic_Bullet_3_C" (1.0 1.0 1.0) _returnvalue)))))

(event `InputAxis|MoveForward` :overrideparent false
  (params (AxisValue :type "Float (single-precision)"))
  ;[1 1 1] Movement
  (`self.AddMovementInput` (`KismetMathLibrary.GetForwardVector` (`KismetMathLibrary.MakeRotator` 0.0 0.0 (.yaw (`self.GetControlRotation`)))) AxisValue))

(event `InputAxis|MoveRight` :overrideparent false
  (params (AxisValue :type "Float (single-precision)"))
  ;[1 1 1] Movement
  (`self.AddMovementInput` (`KismetMathLibrary.GetRightVector` (`KismetMathLibrary.MakeRotator` 0.0 0.0 (.yaw (`self.GetControlRotation`)))) AxisValue))

(event `InputAction|Magic`
  (params (Key :type "Key Structure"))
  (bind _returnvalue (`SceneComponent.K2_GetComponentRotation` (`self.Arrow1`)))
  ;[1 1 1] Magic
  (:`Pressed`
    (switch `int` (`self.Weapon_Number`)
      (:`Default`
        (`self.Shoot Projectile` 5.0 "/Game/BP/Blueprints/Combat/BP_AcidBullet.BP_AcidBullet_C" (0.5 0.5 0.5) _returnvalue :!label _label_2))
      (:`1`
        (goto _label_2))
      (:`2`
        (`self.Shoot Projectile` 1.0 "/Game/BP/Blueprints/Combat/BP_RadiationBullet.BP_RadiationBullet_C" (1.0 1.0 1.0) _returnvalue))
      (:`3`
        (set `self.FlameThrowerActivate` true)))))

(event `InputAction|Dash`
  (params (Key :type "Key Structure"))
  ;[1 1 1] Dash
  (:`Pressed`
    (if (<= (`self.Dash_Count`) 0)
      (`KismetSystemLibrary.Delay` 3.0)
      (set `self.Dash_Count` 3)
      (else
        (`self.Dash` 5.0)
        (set `self.Dash_Count` (- (`self.Dash_Count`) 1))))))

(event `self.FlameThrowerHitBox.OnComponentBeginOverlap`
  (params (OverlappedComponent :type "PrimitiveComponent Object Reference") (OtherActor :type "Actor Object Reference") (OtherComp :type "PrimitiveComponent Object Reference") (OtherBodyIndex :type Integer) (bFromSweep :type Boolean) (SweepResult :type "HitResult Structure (by ref)"))
  ;[1 1 1] Magic
  (if (`self.FlameThrowerActivate`)
    (message `/Game/BP/Blueprints/Combat/BP_Debuff_Interfacer.RadiationDebuff` OtherActor)))

(fn `Dash`
  (params (Dash :type "Float (double-precision)"))
  (`self.LaunchCharacter` (* (`self.GetVelocity`) Dash) false true)
  (set `CharacterMovementComponent.MaxWalkSpeed` 600.0 (`self.CharacterMovement`)))

(fn `Debuf`
  (params (MaxWalkSpeed :type "Float (double-precision)" :default 300.0) (Damage :type "Float (double-precision)"))
  (set `CharacterMovementComponent.MaxWalkSpeed` MaxWalkSpeed (`self.CharacterMovement`))
  (`GameplayStatics.ApplyDamage` (`GameplayStatics.GetPlayerPawn` 0) Damage))

(fn `Flame Thrower Emitter`
  (bind _mesh (`self.Mesh`))
  (bind (_returnvalue_location _returnvalue_rotation) (`KismetMathLibrary.BreakTransform` (`SceneComponent.K2_GetComponentToWorld` _mesh)))
  (`GameplayStatics.SpawnEmitterAttached` "/Game/BP/Blueprints/Combat/Flame.Flame" _mesh "GunSocket" _returnvalue_location _returnvalue_rotation (1.0 1.0 1.0) "SnapToTargetIncludingScale" true "None" false))

(fn `NewFunction_0`
  (bind _mesh (`self.Mesh`))
  (`PrimitiveComponent.SetMaterial` _mesh 0 "/Game/BP/Blueprints/Combat/M_AcidEffect.M_AcidEffect")
  (`PrimitiveComponent.SetMaterial` _mesh 1 "/Game/BP/Blueprints/Combat/M_AcidEffect.M_AcidEffect")
  (`PrimitiveComponent.SetMaterial` _mesh 2 "/Game/BP/Blueprints/Combat/M_AcidEffect.M_AcidEffect")
  (`PrimitiveComponent.SetMaterial` _mesh 3 null)
  (`PrimitiveComponent.SetMaterial` _mesh 4 "/Game/BP/Blueprints/Combat/M_AcidEffect.M_AcidEffect")
  (`PrimitiveComponent.SetMaterial` _mesh 5 "/Game/BP/Blueprints/Combat/M_AcidEffect.M_AcidEffect")
  (`PrimitiveComponent.SetMaterial` _mesh 6 null))

(fn `PlayEffect`
  (params (EmitterTemplate :type "ParticleSystem Object Reference") (SystemTemplate :type "NiagaraSystem Object Reference"))
  (bind _mesh (`self.Mesh`))
  (`GameplayStatics.SpawnEmitterAttached` EmitterTemplate _mesh "None" (`SceneComponent.K2_GetComponentLocation` _mesh))
  (`NiagaraFunctionLibrary.SpawnSystemAttached` SystemTemplate _mesh "None" (0.0 0.0 0.0) (struct) "KeepRelativeOffset"))

(fn `RadiationDebuff`)

(fn `Reloading`
  (set `self.Addition_ammo` (- (`self.Max_ammo`) (`self.Current_ammo`)))
  (if (>= (`self.Capacity_ammo`) (`self.Addition_ammo`))
    (set `self.Current_ammo` (+ (`self.Current_ammo`) (`self.Addition_ammo`)))
    (set `self.Capacity_ammo` (- (`self.Capacity_ammo`) (`self.Addition_ammo`)))
    (else
      (set `self.Current_ammo` (+ (`self.Current_ammo`) (`self.Capacity_ammo`)))
      (set `self.Capacity_ammo` 0.0))))

(fn `RotateFunc`
  (bind (_worldlocation _worlddirection) (`PlayerController.DeprojectMousePositionToWorld` (`GameplayStatics.GetPlayerController` 0)))
  (bind _outhit (`KismetSystemLibrary.LineTraceSingle` _worldlocation (+ _worldlocation (* _worlddirection 5000.0)) "TraceTypeQuery1"))
  (bind (_bblockinghit _binitialoverlap _time _distance _location _impactpoint _normal _impactnormal) (`GameplayStatics.BreakHitResult` _outhit))
  (`KismetSystemLibrary.DrawDebugSphere` (`KismetMathLibrary.MakeVector` (.x _location) (.y _location) (.z _location)) 50.0)
  (`SceneComponent.K2_SetWorldLocationAndRotation` (`self.Cursor to World`) (`KismetMathLibrary.MakeVector` (.x _location) (.y _location) (.z _location)) (`KismetMathLibrary.MakeRotationFromAxes` _impactnormal) false false)
  (bind (_returnvalue_roll _returnvalue_pitch _returnvalue_yaw) (`KismetMathLibrary.BreakRotator` (`KismetMathLibrary.FindLookAtRotation` (`self.K2_GetActorLocation`) (`KismetMathLibrary.MakeVector` (.x _location) (.y _location)))))
  (`self.K2_SetActorRotation` (`KismetMathLibrary.MakeRotator` 0.0 0.0 _returnvalue_yaw)))

(fn `Shoot Projectile`
  (params (`Reqaired Ammo` :type "Float (double-precision)") (`Bullet Actor` :type "Actor Class Reference") (Scale :type "Vector Structure") (`Spawn Transform Rotation` :type "Rotator Structure"))
  (bind _returnvalue_location (`KismetMathLibrary.BreakTransform` (`SceneComponent.K2_GetComponentToWorld` (`self.Arrow1`))))
  (`|ExecutionSequence`
    (:`then_0`
      (if (> (`self.Current_ammo`) 0.0)
        (set `self.Current_ammo` (- (`self.Current_ammo`) `Reqaired Ammo`))
        (set `self.Aim_Location` (`.Location` (`GameplayStatics.BreakHitResult` (`PlayerController.GetHitResultUnderCursorByChannel` (`GameplayStatics.GetPlayerController` 0) "TraceTypeQuery1" true))))
        (`|SpawnActorFromClass` `Bullet Actor` (`KismetMathLibrary.MakeTransform` _returnvalue_location `Spawn Transform Rotation` Scale) "AlwaysSpawn" "OverrideRootScale" null null)
        (else
          (`self.Reloading`))))
    (:`then_1`
      (`self.ShootState`))))

(fn `UserConstructionScript`
  (`self.K2_AttachToComponent` null "GunSocket" "SnapToTarget" "SnapToTarget" "KeepRelative" false))