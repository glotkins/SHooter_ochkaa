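; Enemy bullet actor that damages what it overlaps and then destroys itself, ignoring BP_RangeAI.
; A separate Sphere1 overlap spawns BP_Impact and plays an impact sound at the sphere's location for actors without the Enemy tag.
; BeginPlay prints a debug message, and Tick only casts the player pawn to BP_Character without using it.
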(event `self.ReceiveBeginPlay`
  (`KismetSystemLibrary.PrintString` "shooted" true true (struct :`R` 1.0 :`G` 0.00552 :`A` 1.0)))

(event `self.ReceiveActorBeginOverlap`
  (params (OtherActor :type "Actor Object Reference"))
  (`/Engine/EditorBlueprintResources/StandardMacros.IsValid` OtherActor
    (:`Is Valid`
      (if (not (== OtherActor "/Game/BP/Blueprints/AI/BP_RangeAI.BP_RangeAI"))
        (`GameplayStatics.ApplyDamage` OtherActor 1.0)
        (`self.K2_DestroyActor`)))))

(event `self.ReceiveTick`
  (params (DeltaSeconds :type "Float (single-precision)"))
  (cast `/Game/BP/Blueprints/BP_Character` (`GameplayStatics.GetPlayerPawn` 0)))

(event `self.Sphere1.OnComponentBeginOverlap`
  (params (OverlappedComponent :type "PrimitiveComponent Object Reference") (OtherActor :type "Actor Object Reference") (OtherComp :type "PrimitiveComponent Object Reference") (OtherBodyIndex :type Integer) (bFromSweep :type Boolean) (SweepResult :type "HitResult Structure (by ref)"))
  (bind _returnvalue (`SceneComponent.K2_GetComponentLocation` OverlappedComponent))
  (if (not (`self.ActorHasTag` OtherActor "Enemy"))
    (`|SpawnActorFromClass` "/Game/BP/Blueprints/Combat/BP_Impact.BP_Impact_C" (`KismetMathLibrary.MakeTransform` _returnvalue) "Undefined" "OverrideRootScale" null null)
    (`GameplayStatics.PlaySoundAtLocation` "/Game/BP/Blueprints/Sounds/423106__ogsoundfx__guns-explosions-album-bullet-impact-21.423106__ogsoundfx__guns-explosions-album-bullet-impact-21" _returnvalue (struct) 1.0 1.0 0.0 null null null)))

(fn `UserConstructionScript`)