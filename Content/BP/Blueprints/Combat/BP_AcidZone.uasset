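; BP_AcidZone is a combat acid area that can grow from zero scale on BeginPlay and messages actors that begin overlapping it.
; RadiationDebuff and ElectroDebuff events swap the cube material, stop acid particles and set Rad or Electro flags; radiation also spawns an emitter and replays growth.
; On overlap, the flags select RadAcid, ElectroAcid or, with neither set, ElectroDebuff message, with Rad taking priority.
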(event `self.ReceiveBeginPlay`
  (if (`self.Condition`)
    (bind (_direction _newtrack_0) (`Timeline|Timeline_0`)
      (:`Update`
        (`SceneComponent.SetWorldScale3D` (`self.DefaultSceneRoot`) (`KismetMathLibrary.VLerp` (0.0 0.0 0.0) (1.0 1.0 1.0) _newtrack_0))))))

(event `self.ReceiveActorBeginOverlap`
  (params (OtherActor :type "Actor Object Reference"))
  (bind _output_get (set `self.Objects` (`|MakeArray` OtherActor)))
  (for _array_element _output_get
    (if (`self.Rad`)
      (message `/Game/BP/Blueprints/Combat/BP_Debuff_Interfacer.RadAcid` _array_element)
      (elif (`self.Electro`)
        (message `/Game/BP/Blueprints/Combat/BP_Debuff_Interfacer.ElectroAcid` _array_element)
        (else
          (message `/Game/BP/Blueprints/Combat/BP_Debuff_Interfacer.ElectroDebuff` _array_element))))))

(event `/Game/BP/Blueprints/Combat/BP_Debuff_Interfacer.RadiationDebuff`
  (bind (_returnvalue_location _returnvalue_rotation) (`KismetMathLibrary.BreakTransform` (`SceneComponent.K2_GetComponentToWorld` (`self.Box`))))
  (`GameplayStatics.SpawnEmitterAtLocation` null _returnvalue_location _returnvalue_rotation (1.0 1.0 1.0) false)
  (`PrimitiveComponent.SetMaterial` (`self.Cube`) 0 "/Game/BP/Blueprints/Combat/M_acid_2.M_acid_2")
  (bind (_direction _newtrack_0) (`Timeline|Timeline_1`)
    (:`Update`
      (`SceneComponent.SetWorldScale3D` (`self.DefaultSceneRoot`) (`KismetMathLibrary.VLerp` (0.0 0.0 0.0) (1.0 1.0 1.0) _newtrack_0))
      (`ActorComponent.Deactivate` (`self.Acid_ParticleSystem`))
      (set `self.Rad` true))))

(event `/Game/BP/Blueprints/Combat/BP_Debuff_Interfacer.ElectroDebuff`
  (`PrimitiveComponent.SetMaterial` (`self.Cube`) 0 "/Game/BP/Blueprints/Combat/m_lightning.m_lightning")
  (`KismetSystemLibrary.PrintString` "Hello")
  (`ActorComponent.Deactivate` (`self.Acid_ParticleSystem`))
  (set `self.Electro` true))

(fn `UserConstructionScript`)