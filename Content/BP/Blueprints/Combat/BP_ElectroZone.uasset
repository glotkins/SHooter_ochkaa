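; Electric combat zone actor that sends an electro debuff message to the first actor overlapping it.
; The message is the radiation, acid or plain electro variant, chosen by the Rad and Acid flags.
; AcidDebuff sets Acid, while RadiationDebuff swaps the sphere material, disables the player's flamethrower, spawns a LaserBullet from the player's arrow, clears Rad and destroys the zone.
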(event `self.ReceiveActorBeginOverlap`
  (params (OtherActor :type "Actor Object Reference"))
  (`/Engine/EditorBlueprintResources/StandardMacros.DoOnce` false
    (:`Completed`
      (set `self.Objects` (`|MakeArray` OtherActor))
      (for _ (range 1)
        (if (`self.Rad`)
          (message `/Game/BP/Blueprints/Combat/BP_Debuff_Interfacer.ElectroRad` OtherActor)
          (elif (`self.Acid`)
            (message `/Game/BP/Blueprints/Combat/BP_Debuff_Interfacer.ElectroAcid` OtherActor)
            (else
              (message `/Game/BP/Blueprints/Combat/BP_Debuff_Interfacer.ElectroDebuff` OtherActor))))))))

(event `/Game/BP/Blueprints/Combat/BP_Debuff_Interfacer.RadiationDebuff`
  (`/Engine/EditorBlueprintResources/StandardMacros.DoOnce` false
    (:`Completed`
      (`PrimitiveComponent.SetMaterial` (`self.Sphere`) 0 "/Game/BP/Blueprints/Combat/m_lightning_rad.m_lightning_rad")
      (bind _asbp_character (cast `/Game/BP/Blueprints/BP_Character` (`GameplayStatics.GetPlayerPawn` 0)))
      (set `/Game/BP/Blueprints/BP_Character.FlameThrowerActivate` false _asbp_character)
      (`/Engine/EditorBlueprintResources/StandardMacros.DoOnce` false
        (:`Completed`
          (bind _arrow1 (`/Game/BP/Blueprints/BP_Character.Arrow1` _asbp_character))
          (`|SpawnActorFromClass` "/Game/BP/Blueprints/Combat/LaserBullet.LaserBullet_C" (`KismetMathLibrary.MakeTransform` (`SceneComponent.K2_GetComponentLocation` _arrow1) (`SceneComponent.K2_GetComponentRotation` _arrow1)) "AlwaysSpawn" "OverrideRootScale" null null)
          (set `self.Rad` false)
          (`self.K2_DestroyActor`))))))

(event `/Game/BP/Blueprints/Combat/BP_Debuff_Interfacer.AcidDebuff`
  (params (CountAnim :type Integer) (AnimTime :type "Float (single-precision)"))
  (set `self.Acid` true))

(fn `UserConstructionScript`)