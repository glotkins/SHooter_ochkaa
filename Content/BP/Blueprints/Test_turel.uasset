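; Test turret that tracks the player and fires enemy bullets, becoming damageable when its defender count is zero or less.
; Each Tick, Cube1 smoothly turns toward the player while a debug-drawn line trace checks for BP_Character within 3000 units.
; A hit starts a looping timer, never cleared here, that spawns bullets at Arrow1 after a short delay.
; Defenders are counted only at BeginPlay; sound and recoil-like timeline nodes are disconnected.
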(event `self.ReceiveBeginPlay`
  (set `self.Defenders_Count` (`KismetArrayLibrary.Array_Length` (`self.Defenders `)))
  (set `self.CurrentHP` (`self.CurrentHP`)))

(event `self.ReceiveTick`
  (params (DeltaSeconds :type "Float (single-precision)"))
  (bind _returnvalue (`SceneComponent.K2_GetComponentLocation` (`self.Cube1`)))
  (`|ExecutionSequence`
    (:`then_0`
      (if (<= (`self.Defenders_Count`) 0)
        (set `self.Can be damaged` true)))
    (:`then_1`
      (bind _outhit (`KismetSystemLibrary.LineTraceSingle` :`Start` _returnvalue :`End` (`self.K2_GetActorLocation` (`GameplayStatics.GetPlayerPawn` 0)) :`TraceChannel` "TraceTypeQuery2" :`bTraceComplex` true :`DrawDebugType` "ForOneFrame"))
      (`SceneComponent.K2_SetWorldRotation` (`self.Cube1`) (`KismetMathLibrary.RInterpTo` (`SceneComponent.K2_GetComponentRotation` (`self.Cube1`)) (`KismetMathLibrary.MakeRotator` 0.0 (.pitch (`KismetMathLibrary.FindLookAtRotation` (`SceneComponent.K2_GetComponentLocation` (`self.Cube1`)) (`self.K2_GetActorLocation` (`GameplayStatics.GetPlayerPawn` 0)))) (.yaw (`KismetMathLibrary.FindLookAtRotation` (`SceneComponent.K2_GetComponentLocation` (`self.Cube1`)) (`self.K2_GetActorLocation` (`GameplayStatics.GetPlayerPawn` 0))))) (`self.Delta time`) (`self.Rotation Speed`)) false false)
      (`KismetSystemLibrary.DrawDebugSphere` _returnvalue 3000.0 12 (struct :`R` 1.0 :`G` 0.011936 :`A` 1.0) 1.0)
      (bind (_bblockinghit _binitialoverlap _time _distance _location _impactpoint _normal _impactnormal _physmat _hitactor) (`GameplayStatics.BreakHitResult` _outhit))
      (if (<= _distance 3000.0)
        (bind _output_get (set `self.Targ` _hitactor))
        (cast `/Game/BP/Blueprints/BP_Character` _output_get
          (:`then`
            (`/Engine/EditorBlueprintResources/StandardMacros.DoOnce` false :!label _label
              (:`Completed`
                (`KismetSystemLibrary.K2_SetTimerDelegate` (delegate `shoot`) 0.6 true 0.5))))
          (:`CastFailed`
            (goto _label :!via `Reset`)))))))

(event `shoot`
  (bind (_returnvalue_location _returnvalue_rotation) (`KismetMathLibrary.BreakTransform` (`SceneComponent.K2_GetComponentToWorld` (`self.Arrow1`))))
  (`KismetSystemLibrary.Delay` 0.5)
  (`|SpawnActorFromClass` "/Game/BP/Blueprints/Combat/BP_Basic_Bullet_Enemy.BP_Basic_Bullet_Enemy_C" (`KismetMathLibrary.MakeTransform` _returnvalue_location _returnvalue_rotation (0.3 0.3 0.3)) "AlwaysSpawn" "OverrideRootScale" null null))

(fn `UserConstructionScript`)