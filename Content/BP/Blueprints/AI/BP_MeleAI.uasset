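; BP_MeleAI is a melee AI character with health, debuff reactions and an ammo drop on death.
; Damage sets CurrentHP to damage minus current HP (reversed subtraction); at zero or below, Tick stops movement, then after a delay spawns BP_AMMO and destroys the actor.
; Tick also requests AI Perception prediction of the player.
; Acid temporarily slows it through a DoOnce, radiation applies delayed self-damage with fire, and construction attaches a child actor to the weapon socket.
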(event `self.ReceiveBeginPlay`
  (set `self.Current_HP` (`self.Max_HP`)))

(event `self.ReceiveAnyDamage`
  (params (Damage :type "Float (single-precision)") (DamageType :type "DamageType Object Reference") (InstigatedBy :type "Controller Object Reference") (DamageCauser :type "Actor Object Reference"))
  (set `self.Current_HP` (- Damage (`self.Current_HP`))))

(event `/Game/BP/Blueprints/Combat/BP_Debuff_Interfacer.AcidDebuff`
  (params (CountAnim :type Integer) (AnimTime :type "Float (single-precision)"))
  (bind _charactermovement (`self.CharacterMovement`))
  (`/Engine/EditorBlueprintResources/StandardMacros.DoOnce` false
    (:`Completed`
      (set `CharacterMovementComponent.MaxWalkSpeed` 300.0 _charactermovement)
      (set `self.Effect` 3.0)
      (`KismetSystemLibrary.Delay` 3.0)
      (set `CharacterMovementComponent.MaxWalkSpeed` 600.0 _charactermovement))))

(event `self.ReceiveTick`
  (params (DeltaSeconds :type "Float (single-precision)"))
  (`AISense_Prediction.RequestControllerPredictionEvent` null (`GameplayStatics.GetPlayerController` 0) 1.0)
  ;[1 1 1] СМЭРТЬ
  (if (<= (`self.Current_HP`) 0.0)
    (set `CharacterMovementComponent.MaxWalkSpeed` 0.0 (`self.CharacterMovement`))
    (`KismetSystemLibrary.Delay` 3.0)
    (`|SpawnActorFromClass` "/Game/BP/Blueprints/BP_AMMO.BP_AMMO_C" (`self.GetTransform`) "Undefined" "OverrideRootScale" null null)
    (`self.K2_DestroyActor`)))

(event `RadiationDebuff_1_1`
  (params (Entered :type Boolean))
  (`KismetSystemLibrary.Delay` 0.2)
  (`GameplayStatics.ApplyDamage` self 50.0)
  (`GameplayStatics.SpawnEmitterAttached` "/Game/StarterContent/Particles/P_Fire.P_Fire" (`self.Mesh`)))

(fn `RadiationDebuff`
  (return))

(fn `UserConstructionScript`
  (`SceneComponent.K2_AttachToComponent` (`self.ChildActor`) (`self.Mesh`) "weapon" "KeepRelative" "KeepRelative" "KeepRelative" true))