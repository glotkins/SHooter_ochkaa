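; BP_RangeAI is an AI character with a child actor on its weapon socket and reactions to acid and radiation.
; Acidable sets Effect and temporarily slows walking, firing only once as DoOnce never resets; Radiatinable applies delayed self-damage.
; Damage handling sets CurrentHP to damage minus current HP, an inverted subtraction, with no death logic.
; Every Tick requests an AI prediction event for the first player controller.
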(event `self.ReceiveBeginPlay`
  (set `self.Current_HP` (`self.Max_HP`)))

(event `self.ReceiveAnyDamage`
  (params (Damage :type "Float (single-precision)") (DamageType :type "DamageType Object Reference") (InstigatedBy :type "Controller Object Reference") (DamageCauser :type "Actor Object Reference"))
  (set `self.Current_HP` (- Damage (`self.Current_HP`))))

(event `/Game/BP/Blueprints/Combat/BP_Acid_Interfacer.Acidable`
  (bind _charactermovement (`self.CharacterMovement`))
  (`/Engine/EditorBlueprintResources/StandardMacros.DoOnce` false
    (:`Completed`
      (set `CharacterMovementComponent.MaxWalkSpeed` 300.0 _charactermovement)
      (set `self.Effect` 1.0)
      (`KismetSystemLibrary.Delay` 6.0)
      (set `CharacterMovementComponent.MaxWalkSpeed` 600.0 _charactermovement))))

(event `self.ReceiveTick`
  (params (DeltaSeconds :type "Float (single-precision)"))
  (`AISense_Prediction.RequestControllerPredictionEvent` null (`GameplayStatics.GetPlayerController` 0) 1.0))

(event `/Game/BP/Blueprints/Combat/BP_Acid_Interfacer.Radiatinable`
  (`KismetSystemLibrary.Delay` 0.2)
  (`GameplayStatics.ApplyDamage` self 50.0))

(fn `UserConstructionScript`
  (`SceneComponent.K2_AttachToComponent` (`self.ChildActor`) (`self.Mesh`) "weapon" "KeepRelative" "KeepRelative" "KeepRelative" true))